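; Actor component that sets up a melee attack behaviour on its owner through the Gameplay Ability System.
; Initialize stores a config and grants GA_MeleeCombo to the owner's ability system component with the given input ID, returning the result.
; Without a valid input ID, non-player owners still get the ability, while players only get a printed warning.
; Getters expose the config's trace object types and windup-animation flag.
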(fn `GetObjectTypesToTrace`
  (returns (ObjectTypesToTrace :type "Array of EObjectTypeQuery Enum"))
  (bind _config_objecttypestotrace (break `MeleeAttackComponentConfig` (`self.Config`)))
  (return _config_objecttypestotrace))

(fn `HasWindupAnim`
  (returns (HasWindupAnim :type Boolean))
  (bind (_config_objecttypestotrace _config_haswindupanim) (break `MeleeAttackComponentConfig` (`self.Config`)))
  (return _config_haswindupanim))

(fn `Initialize`
  (params (Config :type "MeleeAttackComponentConfig Structure") (InputID :type Integer :default -1))
  (returns (NewParam :type "GameplayAbilitySpecHandle Structure"))
  (bind _returnvalue (`self.GetOwner`))
  (bind _returnvalue_2 (`AbilitySystemBlueprintLibrary.GetAbilitySystemComponent` (`self.GetOwner`)))
  (set `self.Config` Config)
  (`/Engine/EditorBlueprintResources/StandardMacros.IsValid` _returnvalue_2
    (:`Is Valid`
      (if (>= InputID 0)
        (bind _returnvalue_3 (`AbilitySystemComponent.K2_GiveAbility` _returnvalue_2 "/Game/MLlike/Melee/GA_MeleeCombo.GA_MeleeCombo_C" 0 (`local.InputID`) :!label _label))
        (return _returnvalue_3)
        (else
          ; move this to base class for these behaviours
          (if (`/Game/BPFL_Utils.IsPlayerActorType` _returnvalue)
            (`KismetSystemLibrary.PrintString` (`KismetStringLibrary.Concat_StrStr` (`KismetSystemLibrary.GetDisplayName` _returnvalue) "Initializing a behaviour for the player without passing an inputID - player won't be able to trigger this"))
            (else
              (goto _label))))))))
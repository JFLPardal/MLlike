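; Actor component that gives its owning actor a config-driven shooting attack through the Gameplay Ability System.
; Initialize stores the config and grants GA_Shoot to the owner with the supplied input ID.
; Getters expose aiming and shooting animations and the projectile class, printing warnings when unset.
; Projectile spawn location is a configured skeletal mesh socket nudged along the actor's forward direction, falling back to the actor's location without a mesh.
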(fn `GetAimingAnim`
  (returns (AnimMontage :type "AnimMontage Object Reference"))
  (bind _config_aiminganim (break `ShootingAttackComponentConfig` (`self.Config`)))
  (`/Engine/EditorBlueprintResources/StandardMacros.IsValid` _config_aiminganim
    (:`Is Valid`
      _)
    (:`Is Not Valid`
      (`KismetSystemLibrary.PrintString` (`KismetStringLibrary.Concat_StrStr` (`KismetSystemLibrary.GetDisplayName` (`self.GetOwner`)) " - Getting AimingAnim when none was specified - no anim will be played when aiming"))))
  (return _config_aiminganim))

(fn `GetProjectileSpawnLocation`
  (returns (Location :type "Vector Structure"))
  (locals (bValidSkeletalMesh :type Boolean))
  (bind _returnvalue (`self.GetOwner`))
  (bind (_config_aiminganim _config_shootinganim _config_projectileclass _config_projectilespawnsocketname) (break `ShootingAttackComponentConfig` (`self.Config`)))
  (bind _returnvalue_2 (`Actor.GetComponentByClass` _returnvalue "/Script/Engine.SkeletalMeshComponent"))
  (`/Engine/EditorBlueprintResources/StandardMacros.IsValid` _returnvalue_2
    (:`Is Valid`
      (set `local.bValidSkeletalMesh` true)
      (bind _returnvalue_3 (`SceneComponent.GetSocketLocation` _returnvalue_2 _config_projectilespawnsocketname)))
    (:`Is Not Valid`
      (set `local.bValidSkeletalMesh` false)
      (`KismetSystemLibrary.PrintString` (`KismetStringLibrary.Concat_StrStr` (`KismetSystemLibrary.GetDisplayName` (`self.GetOwner`)) " - No SkeletalMeshComponent - will spawn projectile close to the actor"))))
  (return (select `bool` (`local.bValidSkeletalMesh`) :`false` (`Actor.K2_GetActorLocation` (`self.GetOwner`)) :`true` (+ _returnvalue_3 (`KismetMathLibrary.GreaterGreater_VectorRotator` (* (`KismetMathLibrary.Vector_Forward`) 55.0) (`Actor.K2_GetActorRotation` _returnvalue))))))

(fn `GetProjectileToSpawnClass`
  (returns (ProjectileClass :type "Actor Class Reference"))
  (bind (_config_aiminganim _config_shootinganim _config_projectileclass) (break `ShootingAttackComponentConfig` (`self.Config`)))
  (if (not (`KismetSystemLibrary.IsValidClass` _config_projectileclass))
    (`KismetSystemLibrary.PrintString` (`KismetStringLibrary.Concat_StrStr` (`KismetSystemLibrary.GetDisplayName` (`self.GetOwner`)) " - Getting AimingAnim when none was specified - no anim will be played when aiming")))
  (return _config_projectileclass))

(fn `GetShootingAnim`
  (returns (AnimMontage :type "AnimMontage Object Reference"))
  (bind (_config_aiminganim _config_shootinganim) (break `ShootingAttackComponentConfig` (`self.Config`)))
  (`/Engine/EditorBlueprintResources/StandardMacros.IsValid` _config_shootinganim
    (:`Is Valid`
      _)
    (:`Is Not Valid`
      (`KismetSystemLibrary.PrintString` (`KismetStringLibrary.Concat_StrStr` (`KismetSystemLibrary.GetDisplayName` (`self.GetOwner`)) " - Getting ShootingAnim when none was specified - no anim will be played when shooting"))))
  (return _config_shootinganim))

(fn `Initialize`
  (params (Config :type "ShootingAttackComponentConfig Structure") (InputID :type Integer :default -1))
  (returns (AbilitySpecHandle :type "GameplayAbilitySpecHandle Structure"))
  (set `self.Config` Config)
  (bind _abilityspechandle (`/Game/BPFL_Utils.AddAbilityToActor` (`self.GetOwner`) "/Game/MLlike/Shooting/GA_Shoot.GA_Shoot_C" InputID))
  (return _abilityspechandle))
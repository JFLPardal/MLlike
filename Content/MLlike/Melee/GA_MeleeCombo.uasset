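; Melee combo gameplay ability that roots the character and plays a sectioned attack montage, with separate event handling for enemies.
; Input during notify-driven combo windows advances to the next section; otherwise the ability ends and restores walking.
; Punch events box-trace at the notify's bone location, deduplicate hit actors, replenish owner energy and apply damage.
; Per-step damage comes from the combo attribute set, with a fallback for enemies lacking one.
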(event `self.K2_ActivateAbility`
  (`|ExecutionSequence`
    (:`then_0`
      (bind _ascharacter (cast `Character` (`self.GetAvatarActorFromActorInfo`)))
      (bind _output_get (set `self.ThisCharacter` _ascharacter))
      (`CharacterMovementComponent.DisableMovement` (`Character.CharacterMovement` _output_get))
      (`self.EndTaskIfValid` (`self.WindupSectionFinishedTask`))
      (`self.EndTaskIfValid` (`self.ComboEndedTask`))
      (`self.EndTaskIfValid` (`self.SignalAttackTask`)))
    (:`then_1`
      (set `self.SectionIndex` 0)
      (if (`/Game/BPFL_Utils.IsEnemyActorType` (`self.GetAvatarActorFromActorInfo`))
        (bind _asynctaskproxy (`AbilityTask_WaitGameplayEvent.WaitGameplayEvent` (struct :`TagName` "GameplayEvent.Abilities.Melee.SignalAttack") null)
          (:`then`
            (set `self.SignalAttackTask` _asynctaskproxy)
            (`AbilityTask_PlayMontageAndWait.CreatePlayMontageAndWaitProxy` "None" (`self.AnimationMontage`) :!label _label
              (:`then`
                (`self.StartStep_Event`))
              (:`OnCompleted`
                (`self.K2_EndAbility` :!label _label_2))
              (:`OnInterrupted`
                (goto _label_2))
              (:`OnCancelled`
                (goto _label_2))))
          (:`EventReceived`
            (`self.MontageJumpToSection` "NPCAttack")))
        (else
          (bind _asynctaskproxy_2 (`AbilityTask_WaitGameplayEvent.WaitGameplayEvent` (struct :`TagName` "AnimNotify.MeleeWindupSectionEnded") null)
            (:`then`
              (set `self.WindupSectionFinishedTask` _asynctaskproxy_2)
              (bind _asynctaskproxy_3 (`AbilityTask_WaitGameplayEvent.WaitGameplayEvent` (struct :`TagName` "AnimNotify.MeleeComboEnded") null)
                (:`then`
                  (set `self.ComboEndedTask` _asynctaskproxy_3)
                  (goto _label))
                (:`EventReceived`
                  (`self.MontageStop` 0.1))))
            (:`EventReceived`
              (`self.MontageJumpToSection` "NPCAttack"))))))))

(event `StartStep_Event`
  (`|ExecutionSequence`
    (:`then_0`
      (`self.EndTaskIfValid` (`self.InputTask`))
      (`self.EndTaskIfValid` (`self.ComboWindowOpenedTask`))
      (`self.EndTaskIfValid` (`self.ComboWindowClosedTask`))
      (`self.EndTaskIfValid` (`self.WaitForPunchTask`)))
    (:`then_1`
      (`AnimInstance.Montage_JumpToSection` (`SkeletalMeshComponent.GetAnimInstance` (`Character.Mesh` (`self.ThisCharacter`))) (`|GetArrayItem` (`self.SectionsNames`) (`self.SectionIndex`)) (`self.AnimationMontage`))
      (`|ExecutionSequence`
        (:`then_0`
          (bind _asynctaskproxy (`AbilityTask_WaitInputPress.WaitInputPress` false)
            (:`then`
              (set `self.InputTask` _asynctaskproxy))
            (:`OnPress`
              (if (`self.bComboWindowOpen`)
                (set `self.bInputPressed` true)))))
        (:`then_1`
          (bind _asynctaskproxy_2 (`AbilityTask_WaitGameplayEvent.WaitGameplayEvent` (struct :`TagName` "GameplayEvent.ComboWindowOpened") null)
            (:`then`
              (set `self.ComboWindowOpenedTask` _asynctaskproxy_2))
            (:`EventReceived`
              (set `self.bComboWindowOpen` true))))
        (:`then_2`
          (bind _asynctaskproxy_3 (`AbilityTask_WaitGameplayEvent.WaitGameplayEvent` (struct :`TagName` "GameplayEvent.ComboWindowClosed") null)
            (:`then`
              (set `self.ComboWindowClosedTask` _asynctaskproxy_3))
            (:`EventReceived`
              (`|ExecutionSequence`
                (:`then_0`
                  (if (`self.bInputPressed`)
                    (bind _result (`/Engine/EditorBlueprintResources/StandardMacros.IncrementInt` (`self.SectionIndex`))
                      (:`  `
                        (bind _returnvalue (`KismetArrayLibrary.Array_IsValidIndex` (`self.SectionsNames`) _result))
                        (if _returnvalue
                          (`self.StartStep_Event`)
                          (else
                            (`self.K2_EndAbility`)))))
                    (else
                      (`self.K2_EndAbility`))))
                (:`then_1`
                  (set `self.bInputPressed` false)
                  (set `self.bComboWindowOpen` false))))))
        (:`then_3`
          (bind (_asynctaskproxy_4 _payload) (`AbilityTask_WaitGameplayEvent.WaitGameplayEvent` (struct :`TagName` "GameplayEvent.Punch") null true)
            (:`then`
              (set `self.WaitForPunchTask` _asynctaskproxy_4))
            (:`EventReceived`
              (`self.ApplyDamageToPawnsInRange` (`.OptionalObject` (break `GameplayEventData` _payload)) (`self.SectionIndex`)))))))))

(event `self.K2_OnEndAbility`
  (params (bWasCancelled :type Boolean))
  (`self.MontageStop` 0.2)
  (`CharacterMovementComponent.SetMovementMode` (`Character.CharacterMovement` (`self.ThisCharacter`)) "MOVE_Walking" 0))

(fn `ApplyDamageToPawnsInRange`
  (params (Object :type "Object Object Reference") (CurrentComboStep :type Integer))
  (locals (OwnerActor :type "Actor Object Reference"))
  (bind _asbp_anim_notify_melee_payload (cast `/Game/MLlike/Shooting/BP_AnimNotify_Melee_Payload` Object))
  (bind _output_get (set `local.OwnerActor` (`self.GetAvatarActorFromActorInfo`)))
  (bind _returnvalue (`MLlikeBlueprintUtils.GetActorsFirstInterfaceOfType` "/Game/MLlike/Melee/BPI_MeleeCombat.BPI_MeleeCombat_C" _output_get))
  (bind _asbpi_melee_combat (cast `/Game/MLlike/Melee/BPI_MeleeCombat` _returnvalue))
  (bind _objecttypestotrace (`/Game/MLlike/Melee/BPI_MeleeCombat.GetObjectTypesToTrace` _asbpi_melee_combat))
  (bind _bonelocation (`/Game/MLlike/Shooting/BP_AnimNotify_Melee_Payload.BoneLocation` _asbp_anim_notify_melee_payload))
  (bind _outhits (`KismetSystemLibrary.BoxTraceMultiForObjects` :`Start` _bonelocation :`End` _bonelocation :`HalfSize` (25.0 75.0 10.0) :`Orientation` (`KismetMathLibrary.Conv_VectorToRotator` (`Actor.GetActorForwardVector` _output_get)) :`ObjectTypes` _objecttypestotrace :`DrawTime` 3.0))
  (set `self.TargetDataHandle` (make `GameplayAbilityTargetDataHandle`))
  (for _array_element _outhits
    (bind (_bblockinghit _binitialoverlap _time _distance _location _impactpoint _normal _impactnormal _physmat _hitactor) (`GameplayStatics.BreakHitResult` _array_element))
    ; prevents duplicate actors from being processed - dependent on actor's 'CollisionPreset'
    (if (not (`BlueprintSetLibrary.Set_Contains` (`self.TracedActors`) _hitactor))
      (`BlueprintSetLibrary.Set_Add` (`self.TracedActors`) _hitactor)
      (bind _returnvalue_2 (`AbilitySystemBlueprintLibrary.AppendTargetDataHandle` (`self.TargetDataHandle`) (`AbilitySystemBlueprintLibrary.AbilityTargetDataFromHitResult` _array_element)))
      (set `self.TargetDataHandle` _returnvalue_2)
      (bind _returnvalue_3 (`AbilitySystemBlueprintLibrary.AssignSetByCallerMagnitude` (`self.MakeOutgoingGameplayEffectSpec` "/Game/MLlike/Shooting/GE_ReplenishEnergy.GE_ReplenishEnergy_C") "None" 20.0))
      (`self.K2_ApplyGameplayEffectSpecToOwner` _returnvalue_3)
      (bind _damage (`self.GetDamageToApply` (`self.SectionIndex`)))
      (`/Game/BPFL_Combat.CombatHit` (`local.OwnerActor`) _hitactor _damage)))
  (bind _damage_2 (`self.GetDamageToApply` (`local.CurrentComboStep`)))
  (bind _returnvalue_4 (`AbilitySystemBlueprintLibrary.AssignTagSetByCallerMagnitude` (`self.MakeOutgoingGameplayEffectSpec` "/Game/MLlike/Melee/GE_Melee_Punch.GE_Melee_Punch_C") (struct :`TagName` "Effects.MeleeDamage") _damage_2))
  (`self.K2_ApplyGameplayEffectSpecToTarget` _returnvalue_4 (`self.TargetDataHandle`))
  (`BlueprintSetLibrary.Set_Clear` (`self.TracedActors`)))

(fn `EndTaskIfValid`
  (params (NewParam :type "AbilityTask Object Reference"))
  (`/Engine/EditorBlueprintResources/StandardMacros.IsValid` NewParam
    (:`Is Valid`
      (`GameplayTask.EndTask` NewParam))))

(fn `GetDamageToApply`
  (params (StepIndex :type Integer))
  (returns (Damage :type "Float (double-precision)"))
  (bind _returnvalue (`AbilitySystemComponent.GetAttributeSet` (`self.GetAbilitySystemComponentFromActorInfo`) "/Script/MLlike.MeleeComboAttributeSet"))
  (`/Engine/EditorBlueprintResources/StandardMacros.IsValid` _returnvalue
    (:`Is Valid`
      (bind _returnvalue_2 (`MeleeComboAttributeSet.GetDamageForStep` _returnvalue (select `int` (`local.StepIndex`) :`0` "First" :`1` "Second" :`2` "Third" :!type "EMeleeComboStep Enum")))
      (return _returnvalue_2))
    (:`Is Not Valid`
      ; needed because enemies don't have aattribute sets - remove in the future if this changes
      (return (`self.FallbackDamage`)))))
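; Gameplay ability that makes a character implementing BPI_ProjectileShooter fire a projectile.
; On commit it adds a shot tag, disables movement until the ability ends, then plays the aiming montage and waits for the SignalShooting event.
; Without an aiming montage, it applies GE_Shoot with a set-by-caller energy cost and fires immediately.
; Shoot plays the firing montage and spawns the interface-supplied projectile, passing it the owner's ability system component.
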(event `self.K2_ActivateAbility`
  (bind _returnvalue (`self.GetAvatarActorFromActorInfo`))
  (bind _ascharacter (cast `Character` _returnvalue))
  (bind _returnvalue_2 (`self.K2_CommitAbility`))
  (if _returnvalue_2
    (`|ExecutionSequence`
      (:`then_0`
        (`AbilitySystemBlueprintLibrary.AddLooseGameplayTags` _ascharacter (`BlueprintGameplayTagLibrary.MakeLiteralGameplayTagContainer` (struct :`GameplayTags` (struct :`(TagName` "ActionTaken.Shot")))))
        (`CharacterMovementComponent.DisableMovement` (`Character.CharacterMovement` _ascharacter)))
      (:`then_1`
        (bind _asbpi_projectile_shooter (cast `/Game/Variant_TwinStick/Blueprints/AI/BPI_ProjectileShooter` _ascharacter))
        (bind _animmontage (`/Game/Variant_TwinStick/Blueprints/AI/BPI_ProjectileShooter.GetAimingAnim` _asbpi_projectile_shooter))
        (`/Engine/EditorBlueprintResources/StandardMacros.IsValid` _animmontage
          (:`Is Valid`
            (`AbilityAsync_WaitGameplayEvent.WaitGameplayEventToActor` _ascharacter (struct :`TagName` "GameplayEvent.Abilities.Shoot.SignalShooting")
              (:`then`
                (`Character.PlayAnimMontage` _ascharacter _animmontage 1.0 "None"))
              (:`EventReceived`
                (`self.Shoot` :!label _label)
                (`self.K2_EndAbility`))))
          (:`Is Not Valid`
            (bind _output_get (set `self.OwnerASC` (`AbilitySystemBlueprintLibrary.GetAbilitySystemComponent` _returnvalue)))
            (bind _result (`/Engine/EditorBlueprintResources/StandardMacros.NegateFloat` (`.ReturnValue` (`AbilitySystemComponent.GetGameplayAttributeValue` (`self.OwnerASC`) (struct :`AttributeName` "EnergyCostPerShot" :`Attribute` "/Script/MLlike.ShootingAttributeSet:EnergyCostPerShot" :`AttributeOwner` "/Script/CoreUObject.Class'/Script/MLlike.ShootingAttributeSet'"))))
              (:`  `
                (bind _returnvalue_3 (`AbilitySystemBlueprintLibrary.AssignTagSetByCallerMagnitude` (`AbilitySystemComponent.MakeOutgoingSpec` :`self` _output_get :`GameplayEffectClass` "/Game/MLlike/Shooting/GE_Shoot.GE_Shoot_C") (struct :`TagName` "Abilities.Shoot.EnergyCost") _result))
                (`AbilitySystemComponent.BP_ApplyGameplayEffectSpecToSelf` (`self.OwnerASC`) _returnvalue_3)
                (goto _label)))))))))

(event `self.K2_OnEndAbility`
  (params (bWasCancelled :type Boolean))
  (bind _ascharacter (cast `Character` (`self.GetAvatarActorFromActorInfo`)))
  (`CharacterMovementComponent.SetMovementMode` (`Character.CharacterMovement` _ascharacter) "MOVE_Walking" 0))

(fn `Shoot`
  (bind _returnvalue (`self.GetAvatarActorFromActorInfo`))
  (bind (_returnvalue_location _returnvalue_rotation _returnvalue_scale) (`KismetMathLibrary.BreakTransform` (`Actor.GetTransform` _returnvalue)))
  (bind _asbpi_projectile_shooter (cast `/Game/Variant_TwinStick/Blueprints/AI/BPI_ProjectileShooter` _returnvalue)
    (:`then`
      (`|ExecutionSequence`
        (:`then_0`
          (bind _animmontage (`/Game/Variant_TwinStick/Blueprints/AI/BPI_ProjectileShooter.GetShootingAnim` _asbpi_projectile_shooter))
          (`/Engine/EditorBlueprintResources/StandardMacros.IsValid` _animmontage
            (:`Is Valid`
              (bind _ascharacter (cast `Character` _returnvalue))
              (`Character.PlayAnimMontage` _ascharacter _animmontage 1.0 "None"))))
        (:`then_1`
          (bind _projectileclass (`/Game/Variant_TwinStick/Blueprints/AI/BPI_ProjectileShooter.GetProjectileToSpawnClass` _asbpi_projectile_shooter))
          (bind _location (`/Game/Variant_TwinStick/Blueprints/AI/BPI_ProjectileShooter.GetProjectileSpawnLocation` _asbpi_projectile_shooter))
          (bind _returnvalue_2 (`|SpawnActorFromClass` _projectileclass (`KismetMathLibrary.MakeTransform` _location _returnvalue_rotation _returnvalue_scale) "AlwaysSpawn" "MultiplyWithRoot" null null))
          (bind _asmllike_ability_system_component (cast `MLLikeAbilitySystemComponent` (`AbilitySystemBlueprintLibrary.GetAbilitySystemComponent` _returnvalue)))
          (bind _astwin_stick_projectile (cast `TwinStickProjectile` _returnvalue_2))
          (`TwinStickProjectile.SetOwnerASC` _astwin_stick_projectile _asmllike_ability_system_component))))
    (:`CastFailed`
      (`KismetSystemLibrary.PrintString` "Added GA_Shoot to a character that is not implementing BPI_ProjectileShooter - Can't retrieve projectile to spawn"))))